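; A 2D sprite lift that moves between its origin and EndLocation via a timeline lerp.
; When finished, it waits StopDelay, then runs the opposite way.
; Player overlap with SafetyCollider calls Play or Reverse on an active timeline, but BeginPlay is empty and play-rate setup is unwired.
; The construction script sets sprite color and can preview the end position.
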(event OnComponentBeginOverlap(SafetyCollider)
  (params (OverlappedComponent :type Primitive%20Component%20Object%20Reference) (OtherActor :type Actor%20Object%20Reference) (OtherComp :type Primitive%20Component%20Object%20Reference) (OtherBodyIndex :type Integer) (bFromSweep :type Boolean) (SweepResult :type Hit%20Result%20Structure%20%28by%20ref%29))
  (bind _lifttimeline (Variables|Default|GetLiftTimeline))
  (Utilities|Casting|CastToMycharacter OtherActor)
  (if (Components|Activation|IsActive _lifttimeline)
    (if (Audio|Components|Audio|IsPlaying _lifttimeline)
      (bind (_direction _lerp_alpha) (Timeline|LiftTimeline Play)
        (:Update
          (Transformation|SetRelativeLocation (Variables|Default|GetLiftSprite) (Math|Vector|Lerp(Vector) "0, 0, 0" (Variables|LiftControlls|GetEndLocation) _lerp_alpha) false false))
        (:Finished
          (Utilities|FlowControl|Delay (Variables|LiftControlls|GetStopDelay))
          (switch Utilities|FlowControl|Switch|SwitchonETimelineDirection _direction
            (:Forward
              (CallFunction|LiftBackward))
            (:Backward
              (CallFunction|LiftForward)))))
      (else
        (Timeline|LiftTimeline Reverse)))))

(event Custom|LiftBackward
  (bind (_direction _lerp_alpha) (Timeline|LiftTimeline ReverseFromEnd)
    (:Update
      (Transformation|SetRelativeLocation (Variables|Default|GetLiftSprite) (Math|Vector|Lerp(Vector) "0, 0, 0" (Variables|LiftControlls|GetEndLocation) _lerp_alpha) false false))
    (:Finished
      (Utilities|FlowControl|Delay (Variables|LiftControlls|GetStopDelay))
      (switch Utilities|FlowControl|Switch|SwitchonETimelineDirection _direction
        (:Forward
          (CallFunction|LiftBackward))
        (:Backward
          (CallFunction|LiftForward))))))

(event Custom|LiftForward
  (bind (_direction _lerp_alpha) (Timeline|LiftTimeline PlayFromStart)
    (:Update
      (Transformation|SetRelativeLocation (Variables|Default|GetLiftSprite) (Math|Vector|Lerp(Vector) "0, 0, 0" (Variables|LiftControlls|GetEndLocation) _lerp_alpha) false false))
    (:Finished
      (Utilities|FlowControl|Delay (Variables|LiftControlls|GetStopDelay))
      (switch Utilities|FlowControl|Switch|SwitchonETimelineDirection _direction
        (:Forward
          (CallFunction|LiftBackward))
        (:Backward
          (CallFunction|LiftForward))))))

(event EventBeginPlay)

(fn ConstructionScript
  (bind _liftsprite (Variables|Default|GetLiftSprite))
  (Transformation|SetRelativeLocation _liftsprite (Math|Vector|SelectVector (Variables|LiftControlls|GetEndLocation) "0, 0, 0" (Variables|LiftControlls|GetTestEndLocation)) false false)
  (Sprite|SetSpriteColor _liftsprite (Variables|LiftControlls|GetLiftColor)))